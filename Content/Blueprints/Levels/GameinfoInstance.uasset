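; Game instance that drives the menu flow and multiplayer session handling for a lobby-based game.
; A save-slot check opens either the main menu or first-time options, and most menu widgets are cached for reuse.
; Session events host a listen-server Lobby, join or destroy sessions, with a loading screen during host and join.
; Failures route to DisplayErrorMessage, but it and both error-to-string helpers are empty stubs.
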(event Custom|showMainMenu
  (bind _returnvalue (Game|GetPlayerController 0))
  ;[1 1 1] Show Main menu and Mouse Cursor
  (Utilities|IsValid (Variables|Widgets|Getmainmenuwb)
    (:Is%20Valid
      _)
    (:Is%20Not%20Valid
      (bind _returnvalue_2 (UserInterface|CreateWidget "/Game/Ui/MainMenu/mainmenu.mainmenu_C" _returnvalue))
      (Variables|Widgets|Setmainmenuwb _returnvalue_2)))
  (UserInterface|Viewport|AddtoViewport (Variables|Widgets|Getmainmenuwb) 0)
  (Variables|/Script/Engine.PlayerController|SetbShowMouseCursor _returnvalue true))

(event Custom|ShowHostMenu
  ;[1 1 1] Host game Menu
  (Utilities|IsValid (Variables|Widgets|GetHostMenuWB)
    (:Is%20Valid
      _)
    (:Is%20Not%20Valid
      (bind _returnvalue (UserInterface|CreateWidget "/Game/Ui/MainMenu/hostmenu.hostmenu_C" (Game|GetPlayerController 0)))
      (Variables|Widgets|SetHostMenuWB _returnvalue)))
  (UserInterface|Viewport|AddtoViewport (Variables|Widgets|GetHostMenuWB) 0))

(event Custom|ShozSererMenu
  ;[1 1 1] Show server menu
  (bind _returnvalue (UserInterface|CreateWidget "/Game/Ui/MainMenu/servermenu.servermenu_C" (Game|GetPlayerController 0)))
  (UserInterface|Viewport|AddtoViewport _returnvalue 0))

(event Custom|ShowOptionsMenu
  ;[1 1 1] Show options menu
  (Utilities|IsValid (Variables|Widgets|GetOptionsWB)
    (:Is%20Valid
      _)
    (:Is%20Not%20Valid
      (bind _returnvalue (UserInterface|CreateWidget "/Game/Ui/MainMenu/optionsmenu.optionsmenu_C" (Game|GetPlayerController 0)))
      (Variables|Widgets|SetOptionsWB _returnvalue)))
  (UserInterface|Viewport|AddtoViewport (Variables|Widgets|GetOptionsWB) 0)
  (if (not (Variables|Default|GetCreatedSaveFile))
    (Variables|/Game/Ui/MainMenu/optionsmenu.optionsmenu_C|SetWelcomeMessage (Variables|Widgets|GetOptionsWB) "Visible")))

(event Custom|LaunchLobby
  (params (numberOfPlayers :type Integer) (EnableLan :type Boolean) (ServerName :type Text))
  ;[1 1 1] Launch the lobby
  (Variables|ServerSettings|SetMaxPlayers numberOfPlayers)
  (Variables|ServerSettings|SetServerName ServerName)
  (CallFunction|ShowLoadinscreen)
  (|Session (Game|GetPlayerController 0) (Variables|ServerSettings|GetMaxPlayers) EnableLan
    (:OnSuccess
      (Game|OpenLevel(byName) "Lobby" true "listen"))
    (:OnFailure
      (Utilities|DisplayErrorMessage "Failed to create session, please try again"))))

(event Custom|ShowLoadinscreen
  ;[1 1 1] Show Loading screen
  (Utilities|IsValid (Variables|Widgets|GetLoadingScreenWB)
    (:Is%20Valid
      _)
    (:Is%20Not%20Valid
      (bind _returnvalue (UserInterface|CreateWidget "/Game/Ui/Levels/loadingscreen.loadingscreen_C" (Game|GetPlayerController 0)))
      (Variables|Widgets|SetLoadingScreenWB _returnvalue)))
  (UserInterface|Viewport|AddtoViewport (Variables|Widgets|GetLoadingScreenWB) 0))

(event Custom|JoinServer
  (params (SessionToJoin :type Blueprint%20Session%20Result%20Structure))
  ;[1 1 1] Join Session
  (CallFunction|ShowLoadinscreen)
  (|JoinSession (Game|GetPlayerController 0) SessionToJoin
    (:then
      (Utilities|DisplayErrorMessage "Failed to Join session, please try again"))))

(event Custom|DestroySessionCaller
  (params (PlayerController :type Player%20Controller%20Object%20Reference))
  ;[1 1 1] Destroy Session
  (|DestroySession PlayerController))

(event Custom|SaveGameCheck
  ;[1 1 1] Check for save game
  (bind _returnvalue (SaveGame|DoesSaveGameExist (Variables|Default|GetPlayerSettingsSaved)))
  (if _returnvalue
    (CallFunction|ShowMainMenu)
    (Variables|Default|SetCreatedSaveFile true)
    (else
      (CallFunction|ShowOptionsMenu)
      (Variables|/Script/Engine.PlayerController|SetbShowMouseCursor (Game|GetPlayerController 0) true))))

(event EventHandleNetworkError
  (params (FailureType :type ENetworkFailure%20Enum :default "NetDriverAlreadyExists") (bIsServer :type Boolean))
  ;[1 1 1] Handle Network Errors
  (if bIsServer
    _
    (else
      _))
  (Utilities|DisplayErrorMessage (CallFunction|NetErrorTostring FailureType)))

(event EventHandleTravelError
  (params (FailureType :type ETravelFailure%20Enum :default "NoLevel"))
  ;[1 1 1] Handle Travel Error
  (Utilities|DisplayErrorMessage (CallFunction|TravelErorrorTostring FailureType)))

(fn NetErrorTostring
  (params (FailureType :type ENetworkFailure%20Enum :default "NetDriverAlreadyExists"))
  (return ""))

(fn TravelErorrorTostring
  (params (FailureType :type ETravelFailure%20Enum :default "NoLevel"))
  (return ""))